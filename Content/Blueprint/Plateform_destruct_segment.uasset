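; Destructible platform segment that shakes and breaks apart when its hitbox is overlapped, then respawns.
; A Rumbling timeline offsets the anchored DestructivePlat, then a MasterField actor spawns at the Cible position, presumably to fracture it.
; After a delay, a Desapear timeline scales the pieces before the platform, hitbox and field root components are destroyed.
; Once TimeBeforeRespawn elapses, it spawns a fresh anchored copy of itself at the saved location, without destroying the old actor.
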(event OnComponentBeginOverlap(Hitbox)
  (params (OverlappedComponent :type Primitive%20Component%20Object%20Reference) (OtherActor :type Actor%20Object%20Reference) (OtherComp :type Primitive%20Component%20Object%20Reference) (OtherBodyIndex :type Integer) (bFromSweep :type Boolean) (SweepResult :type Hit%20Result%20Structure%20%28by%20ref%29))
  (bind _newtrack_3 (Timeline|Rumbling Play)
    (:Update
      (Transformation|SetRelativeLocation (Variables|Default|GetDestructive_plat) (+ _newtrack_3 (Variables|Default|GetPosition_Ini)) false false))
    (:Finished
      (bind _returnvalue (Game|SpawnActorfromClass "/Game/Blueprint/MasterField.MasterField_C" (Math|Conversions|ToTransform(Vector) (Variables|Default|GetPosition_Cible)) "Undefined" "MultiplyWithRoot" 0 0))
      (Utilities|FlowControl|Delay 5.0)
      (bind _newtrack_0 (Timeline|Desapear Play)
        (:Update
          (Transformation|SetWorldScale3D (Variables|Default|GetDestructive_plat) (* (Class|KismetMathLibrary|VectorGetSignVector "1.000000,1.000000,1.000000") _newtrack_0)))
        (:Finished
          (Components|DestroyComponent (Variables|Default|GetDestructive_plat))
          (Components|DestroyComponent (Variables|Default|GetHitbox))
          (Components|DestroyComponent (Variables|/Script/Engine.Actor|GetRootComponent _returnvalue))
          (Utilities|FlowControl|Delay (Variables|Default|GetTime%20before%20respawn))
          (bind _returnvalue_2 (Game|SpawnActorfromClass "Plateform_destruct_segment_C" (Variables|Default|GetPosition_plat) "Undefined" "MultiplyWithRoot" 0 0))
          (Class|GeometryCollectionComponent|SetAnchoredbyIndex (Variables|Plateform_destruct_segment_C|GetDestructive_plat _returnvalue_2) 0 true))))))

(event Collision|EventActorBeginOverlap
  (params (OtherActor :type Actor%20Object%20Reference)))

(event EventBeginPlay
  (Variables|Default|SetPosition_Cible (Transformation|GetWorldLocation (Variables|Default|Getcible)))
  (Class|GeometryCollectionComponent|SetAnchoredbyIndex (Variables|Default|GetDestructive_plat) 0 true)
  (Variables|Default|SetPosition_plat (Math|Conversions|ToTransform(Vector) (Transformation|GetWorldLocation (Variables|Default|GetDefaultSceneRoot))))
  (Variables|Default|SetPosition_Ini (Variables|/Script/Engine.SceneComponent|GetRelativeLocation (Variables|Default|GetDestructive_plat))))

(fn ConstructionScript)