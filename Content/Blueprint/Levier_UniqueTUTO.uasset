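; Tutorial lever, a single interactable that the player pulls with the Interaction input.
; A Box overlap enables input and shows a prompt widget, which turns to face the camera every tick; leaving the box reverses both.
; Interaction sets the Valeur flag and plays a timeline that rotates the movable lever part.
; The lever sound spawns on every timeline update rather than once per pull.
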(event OnComponentBeginOverlap(Box)
  (params (OverlappedComponent :type Primitive%20Component%20Object%20Reference) (OtherActor :type Actor%20Object%20Reference) (OtherComp :type Primitive%20Component%20Object%20Reference) (OtherBodyIndex :type Integer) (bFromSweep :type Boolean) (SweepResult :type Hit%20Result%20Structure%20%28by%20ref%29))
  (Input|EnableInput (Game|GetPlayerController 0))
  (Rendering|SetVisibility (Variables|Default|GetWidget) true false))

(event OnComponentEndOverlap(Box)
  (params (OverlappedComponent :type Primitive%20Component%20Object%20Reference) (OtherActor :type Actor%20Object%20Reference) (OtherComp :type Primitive%20Component%20Object%20Reference) (OtherBodyIndex :type Integer))
  (Input|DisableInput (Game|GetPlayerController 0))
  (Rendering|SetVisibility (Variables|Default|GetWidget) false false))

(event EventTick
  (params (DeltaSeconds :type Float%20%28single-precision%29))
  (Transformation|SetWorldRotation (Variables|Default|GetWidget) (Math|Rotator|FindLookatRotation (Transformation|GetWorldLocation (Variables|Default|GetWidget)) (Transformation|GetActorLocation (Game|GetPlayerCameraManager 0))) false false))

(event Input|ActionEvents|InputActionInteraction
  (params (Key :type Key%20Structure :default "None"))
  (:Pressed
    (Variables|Default|SetValeur true)
    (bind _levier_anim (Timeline|Levier Play)
      (:Update
        (Transformation|SetRelativeRotation (Variables|Default|GetLevier_amovible) (Math|Rotator|Lerp(Rotator) "0.000000,90.000000,0.000000" "-90.000000,90.000000,0.000000" _levier_anim) false false)
        (Audio|SpawnSound2D "/Game/Sound/Lever_mixage_final.Lever_mixage_final" 3.0 1.0 0.0 0)))))

(fn ConstructionScript)