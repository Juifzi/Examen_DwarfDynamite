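; Automatic moving platform actor that shuttles back and forth between its Cube's starting position and a Cible target.
; BeginPlay caches both positions and the unit direction between them, then Tick moves the whole actor along it at Vitesse, without sweep.
; Vitesse flips sign at either end, detected by comparing position vector lengths from world origin rather than distance travelled along the path.
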(event EventBeginPlay
  (Variables|Default|SetPosition%20Cube (Transformation|GetWorldLocation (Variables|Default|GetCube)))
  (Variables|Default|SetPosition%20cible (Transformation|GetWorldLocation (Variables|Default|GetCible)))
  (Variables|Default|SetDirection (Math|Vector|GetUnitDirection(Vector) (Variables|Default|GetPosition%20Cube) (Variables|Default|GetPosition%20cible))))

(event EventTick
  (params (DeltaSeconds :type Float%20%28single-precision%29))
  (Transformation|SetActorLocation (+ (* DeltaSeconds (Variables|Default|GetVitesse) (Variables|Default|GetDirection)) (Transformation|GetActorLocation)) false false)
  (if (>= (Variables|Default|GetVitesse) 0.0)
    (if (not (>= (- (Math|Vector|VectorLength (Variables|Default|GetPosition%20cible)) (Math|Vector|VectorLength (Transformation|GetWorldLocation (Variables|Default|GetCube)))) 0.0))
      (Variables|Default|SetVitesse (* (Variables|Default|GetVitesse) -1.0)))
    (elif (not (>= (- (Math|Vector|VectorLength (Transformation|GetWorldLocation (Variables|Default|GetCube))) (Math|Vector|VectorLength (Variables|Default|GetPosition%20Cube))) 0.0))
      (Variables|Default|SetVitesse (* (Variables|Default|GetVitesse) -1.0)))))

(fn ConstructionScript)