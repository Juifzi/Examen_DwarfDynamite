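; Destructible platform actor that destroys itself when something overlaps its Hitbox and spawns a replacement when the overlap ends.
; Begin overlap sets a timer with TimeBeforeDelete, then destroys the actor immediately.
; End overlap sets a timer with TimeBeforeRespawn, then immediately spawns a new Plateform_destructive at the stored Platform's world location.
; Neither timer names a function, so neither delay gates destruction or respawn.
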(event OnComponentBeginOverlap(Hitbox)
  (params (OverlappedComponent :type Primitive%20Component%20Object%20Reference) (OtherActor :type Actor%20Object%20Reference) (OtherComp :type Primitive%20Component%20Object%20Reference) (OtherBodyIndex :type Integer) (bFromSweep :type Boolean) (SweepResult :type Hit%20Result%20Structure%20%28by%20ref%29))
  (Utilities|Time|SetTimerbyFunctionName 0 "" (Variables|Default|GetTime%20before%20delete))
  (Variables|Default|SetPlatform (Variables|Default|GetPlatform))
  (Actor|DestroyActor))

(event OnComponentEndOverlap(Hitbox)
  (params (OverlappedComponent :type Primitive%20Component%20Object%20Reference) (OtherActor :type Actor%20Object%20Reference) (OtherComp :type Primitive%20Component%20Object%20Reference) (OtherBodyIndex :type Integer))
  (Utilities|Time|SetTimerbyFunctionName 0 "" (Variables|Default|GetTime%20before%20respawn))
  (Game|SpawnActorfromClass "Plateform_destructive_C" (Math|Conversions|ToTransform(Vector) (Transformation|GetWorldLocation (Variables|Default|GetPlatform))) "Undefined" "MultiplyWithRoot" 0 0))

(event EventBeginPlay)

(event Collision|EventActorBeginOverlap
  (params (OtherActor :type Actor%20Object%20Reference)))

(event EventTick
  (params (DeltaSeconds :type Float%20%28single-precision%29)))

(fn ConstructionScript)